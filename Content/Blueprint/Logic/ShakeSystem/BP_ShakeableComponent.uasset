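; An actor component that shakes its owning actor by tweening its location when the Shake event fires.
; BeginPlay caches the owner's location; Shake calls the parent implementation and tweens from that origin along OriginalDelta scaled by strength.
; A custom curve shapes the motion over half of ShakeTime, with both strength and duration randomized by up to 30 percent either way.
; A randomized strength value is also printed for debugging.
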(event EventShake
  (params (ShakeStrength :type Float%20%28single-precision%29))
  (bind _returnvalue (* ShakeStrength 0.3))
  (bind _originalactorlocation (Variables|Default|GetOriginalActorLocation))
  (bind _shaketime (Variables|Default|GetShakeTime))
  (bind _returnvalue_2 (* _returnvalue -1.0))
  (bind _returnvalue_3 (* _shaketime 0.3))
  (bind _returnvalue_4 (Math|Random|RandomFloatinRange _returnvalue_2 _returnvalue))
  (bind _returnvalue_5 (+ ShakeStrength _returnvalue_4))
  (|CallParentFunction ShakeStrength)
  (Development|PrintString (Utilities|String|ToString(Float) _returnvalue_5))
  (bind _value (|TweenVectorCustomCurve _originalactorlocation (+ _originalactorlocation (* (Variables|Default|GetOriginalDelta) _returnvalue_5)) (/ (+ (Variables|Default|GetShakeTime) (Math|Random|RandomFloatinRange (* _returnvalue_3 -1.0) _returnvalue_3)) 2.0) (Variables|Default|GetShakeCurve))
    (:ApplyEasing
      (Transformation|SetActorLocation (Components|GetOwner) _value false false))))

(event EventBeginPlay
  (Variables|Default|SetOriginalActorLocation (Transformation|GetActorLocation (Components|GetOwner))))