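; BP_HUD_Brick is the HUD for the brick game, responsible for setting up its canvas widget.
; CreateWidgets creates a WBP_BrickGameCanvas for the player controller, stores it and adds it to the viewport.
; InitializeWidgets passes the UI and game event holders into that canvas and returns whether its initialization succeeded.
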(fn ConstructionScript)

(fn CreateWidgets
  (bind _returnvalue (UserInterface|CreateWidget "/Game/Blueprint/UI/BrickGame/WBP_BrickGameCanvas.WBP_BrickGameCanvas_C" (Variables|Default|GetPlayerController)))
  (bind _output_get (Variables|Default|SetBrickGameCanvas _returnvalue))
  (UserInterface|Viewport|AddtoViewport _output_get 0)
  (return true))

(fn InitializeWidgets
  (bind _success (Default|InitBrickGameCanvas (Variables|Default|GetBrickGameCanvas) (Variables|Default|GetUIEventHolder) (Variables|Default|GetGameEventHolder)))
  (if _success
    (return true)
    (else
      (return false))))