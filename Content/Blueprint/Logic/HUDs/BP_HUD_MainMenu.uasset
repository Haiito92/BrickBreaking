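; BP_HUD_MainMenu is the main menu HUD, which owns and drives the WBP_MainMenuCanvas widget.
; It extends the parent's CreateWidgets step to add the canvas to the viewport, logging an on-screen error if creation fails.
; InitializeWidgets passes the UI event holder to the canvas once the parent step succeeds, and StartHUD starts the canvas.
; Both setup overrides return success or failure.
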(event EventStartHUD
  (Default|StartMainMenuCanvas (Variables|Default|GetMainMenuCanvas)))

(fn ConstructionScript)

(fn InitializeWidgets
  (bind _returnvalue (|CallParentFunction))
  (if _returnvalue
    (Default|InitMainMenuCanvas (Variables|Default|GetMainMenuCanvas) (Variables|Default|GetUIEventHolder))
    (return true)
    (else
      (return false))))

(fn CreateWidgets
  (bind _returnvalue (|CallParentFunction))
  (if _returnvalue
    (bind _returnvalue_2 (UserInterface|CreateWidget "/Game/Blueprint/UI/MainMenu/WBP_MainMenuCanvas.WBP_MainMenuCanvas_C" (Variables|Default|GetPlayerController)))
    (Utilities|IsValid _returnvalue_2
      (:Is%20Valid
        (bind _output_get (Variables|Default|SetMainMenuCanvas _returnvalue_2))
        (UserInterface|Viewport|AddtoViewport _output_get 0)
        (return true))
      (:Is%20Not%20Valid
        (Class|LittleDebugLibrary|AddonScreenDebugMessage "(TagName=\"GameLoop\")" "Error" "[BP_HUD_MainMenu] Failed to create main menu canvas!" "(R=1.000000,G=0.106892,B=0.101481,A=1.000000)" 3.0)
        (return false)))
    (else
      (return false))))