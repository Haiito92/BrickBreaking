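; BP_ExplosiveBrick is a brick that explodes when broken, hitting breakable neighbors along its four horizontal axes.
; On initialization it derives the blast range from its box collision extent and caches the right, left, forward and back directions.
; Breaking fires visibility multi-traces and sends a hit message once to each Breakable actor, then launches a world shake before the parent break.
; An Exploded flag keeps the blast from repeating.
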(event EventInitializeBrick
  (bind _returnvalue (Transformation|GetActorRightVector))
  (bind _returnvalue_2 (Transformation|GetActorForwardVector))
  (bind _explosiondirections (Variables|Default|GetExplosionDirections))
  (|CallParentFunction)
  (Variables|Default|SetExplosionRange (* (.x (Components|Box|GetScaledBoxExtent (Variables|Default|GetBoxCollision))) 1.5))
  (Utilities|Array|AddUnique _explosiondirections _returnvalue)
  (Utilities|Array|AddUnique _explosiondirections (* _returnvalue -1.0))
  (Utilities|Array|AddUnique _explosiondirections _returnvalue_2)
  (Utilities|Array|AddUnique _explosiondirections (* _returnvalue_2 -1.0)))

(event EventBreak
  (|CallParentFunction))

(event EventBreak
  (bind _returnvalue (Transformation|GetActorLocation))
  (if (not (Variables|Default|GetExploded))
    (Variables|Default|SetExploded true)
    (Utilities|Array|Clear (Variables|Default|GetHitActors))
    (for _array_element (Variables|Default|GetExplosionDirections)
      (bind _outhits (Collision|MultiLineTraceByChannel _returnvalue (+ _returnvalue (* _array_element (Variables|Default|GetExplosionRange))) "TraceTypeQuery1" true 0 "None"))
      (for _array_element_2 _outhits
        (if (Math|Boolean|ANDBoolean (Utilities|IsValid (.HitActor (Collision|BreakHitResult _array_element_2))) (not (Utilities|Array|ContainsItem (Variables|Default|GetHitActors) (.HitActor (Collision|BreakHitResult _array_element_2)))) (Utilities|DoesObjectImplementInterface (.HitActor (Collision|BreakHitResult _array_element_2)) "/Script/BrickBreaking.Breakable"))
          (Class|Breakable|Hit(Message) (.HitActor (Collision|BreakHitResult _array_element_2)))
          (Utilities|Array|AddUnique (Variables|Default|GetHitActors) (.HitActor (Collision|BreakHitResult _array_element_2))))))
    (Class|ShakeWorldSubsystem|LaunchShake (Subsystems|GetShakeWorldSubsystem) (Variables|Default|GetExplosionStrengh))
    (|CallParentFunction)))

(fn ConstructionScript)