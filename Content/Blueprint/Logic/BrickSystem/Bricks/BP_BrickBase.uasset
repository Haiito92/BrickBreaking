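; BP_BrickBase is the base brick Blueprint, providing audio and particle feedback for hits and breaking.
; BreakableHit plays the hit sound and spawns the hit effect at the brick's location, only while Health is above zero and each asset is valid.
; Break plays the break sound with brick attenuation and spawns the break effect, without validity checks.
; This graph neither changes Health nor destroys the actor.
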(event EventBreakableHit
  (bind _returnvalue (Transformation|GetActorLocation))
  (if (> (Variables|Default|GetHealth) 0)
    (Utilities|FlowControl|Sequence
      (:then_0
        (bind _hitsound (Variables|Brick|Juicyness|GetHitSound)
          (:then
            (Audio|PlaySoundatLocation _hitsound _returnvalue "0, 0, 0" 1.0 1.0 0.0 "/Game/Assets/Sounds/Attenuations/SA_Brick.SA_Brick" 0 0 0))
          (:else)))
      (:then_1
        (bind _hiteffect (Variables|Brick|Juicyness|GetHitEffect)
          (:then
            (Niagara|SpawnSystematLocation _hiteffect _returnvalue))
          (:else))))))

(event EventBreak
  (bind _returnvalue (Transformation|GetActorLocation))
  (Audio|PlaySoundatLocation (Variables|Brick|Juicyness|GetBreakSound) _returnvalue "0, 0, 0" 1.0 1.0 0.0 "/Game/Assets/Sounds/Attenuations/SA_Brick.SA_Brick" 0 0 0)
  (Niagara|SpawnSystematLocation (Variables|Brick|Juicyness|GetBreakEffect) _returnvalue))

(fn ConstructionScript)